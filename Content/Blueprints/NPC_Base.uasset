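; NPC_Base is a base Blueprint for interactable NPCs with a floating name label and a dialogue hook.
; The construction script copies CharacterName into the label, and SetInteractableState toggles its visibility.
; Interact prints a debug message and creates a W_Dialogue widget, without adding it to the viewport here.
; ConversationClosed forwards a closed message to InteractInstagator, which this file never assigns.
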(event `/Game/Blueprints/BPI_Interactable.Set Interactable State`
  (params (CanShowInteract :type Boolean))
  (if CanShowInteract
    (`SceneComponent.SetVisibility` (`self.Txt_CharacterName`) true true)
    (else
      (`SceneComponent.SetVisibility` (`self.Txt_CharacterName`) false false))))

(event `/Game/Blueprints/BPI_Interactable.Interact`
  (params (`Instigator ` :type "Actor Object Reference"))
  (`KismetSystemLibrary.PrintString` "interacted w npc")
  (`|CreateWidget` "/Game/Blueprints/NewFolder/W_Dialogue.W_Dialogue_C" null null))

(event `/Game/Blueprints/BPI_Interactable.ConversationClosed`
  (message `/Game/Blueprints/BPI_Interactable.ConversationClosed` (`self.InteractInstagator`)))

(fn `UserConstructionScript`
  (`TextRenderComponent.K2_SetText` (`self.Txt_CharacterName`) (`self.CharacterName`)))