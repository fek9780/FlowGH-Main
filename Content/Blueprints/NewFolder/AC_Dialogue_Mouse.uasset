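; Dialogue component for the Mouse NPC, scripting a branching conversation in which it asks the player for cheese.
; The Dialogue function switches on DialogueTreeIndex and chains inherited AddDialogue calls, branching on the returned option index when State is Pass Through.
; Giving cheese advances to a second tree with a random follow-up line, while refusals remove or clear dialogue progress.
; BeginPlay only prints a debug string.
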(event `self.ReceiveBeginPlay`
  (`parent.ReceiveBeginPlay`)
  (`KismetSystemLibrary.PrintString` "BeginPlay on component called'"))

(fn `Dialogue`
  (bind _array (`|MakeArray` "yes" "No" :!type "Text"))
  (switch `int` (`self. Dialogue Tree Index`)
    (:`0`
      (set `self.Option Text` _array)
      (bind (_state _option_index) (`self.Add Dialogue` "Mouse" "Hi, do you have any cheese" _array "/Engine/VREditor/Sounds/UI/Camera_Shutter.Camera_Shutter" "/Game/Characters/Mannequins/Anims/Pistol/MM_Pistol_Fire_Montage.MM_Pistol_Fire_Montage"))
      (`/Game/Blueprints/NewFolder/W_Dialogue.UpdateDialogueText` (`self.Dialogue Widget`) (`self. Dialogue Index`) "" "" (`self.Option Text`))
      (`KismetSystemLibrary.PrintString` "Options Text Length")
      (switch `/Game/Blueprints/NewFolder/Enum_Dialogue_State` _state
        (:`NewEnumerator0`
          (switch `int` _option_index
            (:`0`
              (set `self. Dialogue Index` 0)
              (bind (_state_2 _option_index_2) (`self.Add Dialogue` "" "Ah, thats great news. Can I have some?" (`|MakeArray` "Give Cheese" "Keep Cheese" :!type "Text") "/Engine/EngineSounds/1kSineTonePing.1kSineTonePing"))
              (switch `/Game/Blueprints/NewFolder/Enum_Dialogue_State` _state_2
                (:`NewEnumerator0`
                  (switch `int` _option_index_2
                    (:`0`
                      (bind _state_3 (`self.Add Dialogue` "" "Thank you, your so kind!" (`|MakeArray` "Continue" :!type "Text")))
                      (switch `/Game/Blueprints/NewFolder/Enum_Dialogue_State` _state_3
                        (:`NewEnumerator0`
                          (`self.Set Dialogue Tree Index` 1)
                          (`self.Closed Conversation`))))
                    (:`1`
                      (bind _state_4 (`self.Add Dialogue` "" "You big meanie!" (`|MakeArray` "Yes" :!type "Text")))
                      (switch `/Game/Blueprints/NewFolder/Enum_Dialogue_State` _state_4
                        (:`NewEnumerator0`
                          (`self.Remove Dialogue Progress` 2)
                          (`self.Closed Conversation`))))))))
            (:`1`
              (bind _state_5 (`self.Add Dialogue` "" "Awww, thats a shame, I really wanted some cheese." (`|MakeArray` "Continue." :!type "Text")))
              (switch `/Game/Blueprints/NewFolder/Enum_Dialogue_State` _state_5
                (:`NewEnumerator0`
                  (`self.Clear Dialogue Progress`)
                  (`self.Closed Conversation`))))))))
    (:`1`
      (bind _state_6 (`self.Add Dialogue` "" (select `int` (`KismetMathLibrary.RandomIntegerInRange` 0 1) :`0` "Your such a nice person." :`1` "Nomm Nomm" :!type "Text")))
      (switch `/Game/Blueprints/NewFolder/Enum_Dialogue_State` _state_6
        (:`NewEnumerator0`
          (`self.Clear Dialogue Progress`)
          (`self.Closed Conversation`))))))