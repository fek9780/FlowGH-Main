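; Blacksmith dialogue component that gives Morning, Afternoon and Night conversations, including a bread request on the Afternoon branch.
; OpenConversation selects the branch from the player character's TimeOfDay, but its index math only yields Morning or Night, leaving Afternoon unreachable.
; Dialogue builds branching lines and choices through the parent's AddDialogue and progress functions, setting HasGivenBread on handover.
; The has-bread check is hardcoded true, with no inventory lookup.
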(fn `Dialogue`
  (`parent.Dialogue`)
  (switch `name` (`self. Active Dialogue Branch`)
    (:`Morning`
      (bind _state (`self.Add Dialogue` "" "Good Morning." (`|MakeArray`)))
      (switch `/Game/Blueprints/NewFolder/Enum_Dialogue_State` _state
        (:`NewEnumerator0`
          (`self.Clear Dialogue Progress`)
          (`self.Closed Conversation`))))
    (:`Afternoon`
      (if (`self.Has given bread?`)
        (bind _state_2 (`self.Add Dialogue` "" "Thank you for the bread." (`|MakeArray`)))
        (switch `/Game/Blueprints/NewFolder/Enum_Dialogue_State` _state_2
          (:`NewEnumerator0`
            (`self.Clear Dialogue Progress`)
            (`self.Closed Conversation`)))
        (else
          (bind (_state_3 _option_index) (`self.Add Dialogue` "" "I want some bread I havent eaten can you get me some?" (`|MakeArray` "sure" "i cant" :!type "Text")))
          (switch `/Game/Blueprints/NewFolder/Enum_Dialogue_State` _state_3
            (:`NewEnumerator0`
              (switch `int` _option_index
                (:`0`
                  (`self.Add Dialogue` "" "Great Come speak to me when you have the bread" (`|MakeArray`))
                  (switch `/Game/Blueprints/NewFolder/Enum_Dialogue_State` "NewEnumerator0"
                    (:`NewEnumerator0`
                      (if true
                        (bind (_state_4 _option_index_2) (`self.Add Dialogue` "" "Ah I see you have bread can I have it please?" (`|MakeArray` "yes" "no" :!type "Text")))
                        (switch `/Game/Blueprints/NewFolder/Enum_Dialogue_State` _state_4
                          (:`NewEnumerator0`
                            (switch `int` _option_index_2
                              (:`0`
                                (`self.Add Dialogue` "" "Ahh wonderfull I love me some good bread" (`|MakeArray`))
                                (switch `/Game/Blueprints/NewFolder/Enum_Dialogue_State` "NewEnumerator0"
                                  (:`NewEnumerator0`
                                    (`self.Clear Dialogue Progress`)
                                    (`self.Closed Conversation`))
                                  (:`NewEnumerator1`
                                    (set `self.Has given bread?` true))))
                              (:`1`
                                (`self.Add Dialogue` "" "Oh okay speak to me if you change your mind" (`|MakeArray`))
                                (switch `/Game/Blueprints/NewFolder/Enum_Dialogue_State` "NewEnumerator0"
                                  (:`NewEnumerator0`
                                    (`self.Remove Dialogue Progress` 0)
                                    (`self.Closed Conversation`)))))))
                        (else
                          (`self.Add Dialogue` "" "Great Come speak to me when you have the bread" (`|MakeArray`))
                          (switch `/Game/Blueprints/NewFolder/Enum_Dialogue_State` "NewEnumerator0"
                            (:`NewEnumerator0`
                              (`self.Remove Dialogue Progress` 0)
                              (`self.Closed Conversation`))))))))
                (:`1`
                  (bind _state_5 (`self.Add Dialogue` "" "ahh okay speak to me if you change your mind" (`|MakeArray`)))
                  (switch `/Game/Blueprints/NewFolder/Enum_Dialogue_State` _state_5
                    (:`NewEnumerator0`
                      (`self.Clear Dialogue Progress`)
                      (`self.Closed Conversation`))))))))))
    (:`Night`
      (`self.Add Dialogue` "" "ahh Im trying to sleep leave me alone" (`|MakeArray`))
      (switch `/Game/Blueprints/NewFolder/Enum_Dialogue_State` "NewEnumerator0"
        (:`NewEnumerator0`
          (`self.Clear Dialogue Progress`)
          (`self.Closed Conversation`))))))

(fn `Open Conversation`
  (bind _interactinstigator (message `/Game/Blueprints/BPI_Interactable.GetInteractionInstigator` (`self.GetOwner`)))
  (bind _asbp_third_person_character (cast `/Game/Blueprints/BP_ThirdPersonCharacter` _interactinstigator))
  (bind (_time_of_day_days _time_of_day_hours) (`KismetMathLibrary.BreakTimespan` (`/Game/Blueprints/BP_ThirdPersonCharacter.Time of Day` _asbp_third_person_character)))
  (`self.Set Dialogue Branch` (select `int` (+ (`KismetMathLibrary.Conv_BoolToInt` (and (>= _time_of_day_hours 5) (< _time_of_day_hours 15))) (* (`KismetMathLibrary.Conv_BoolToInt` (and (<= _time_of_day_hours 0) (> _time_of_day_hours 22))) 0)) :`0` "Night" :`1` "Morning" :`2` "Afternoon" :!type "Name"))
  (`parent.Open Conversation`))